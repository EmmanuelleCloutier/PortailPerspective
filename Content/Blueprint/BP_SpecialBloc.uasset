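; BP_SpecialBloc is a block actor that prints debug messages when it spawns and when it is destroyed.
; It declares a JumpPortal event taking a target location and rotation, but the event is unwired and does nothing.
; Disconnected portal logic would teleport the block to that transform and redirect its existing speed along the new forward vector.
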(event `self.ReceiveBeginPlay`
  (`KismetSystemLibrary.PrintString` "cube spawned"))

(event `self.ReceiveDestroyed`
  (`KismetSystemLibrary.PrintString` "cube destroy"))

(event `/Game/Blueprint/Portal/BPI_PortalJumper.JumpPortal`
  (params (TargetLocation :type "Vector Structure") (TargetRotation :type "Rotator Structure"))
  ;[1 1 1] To Traverse Portal
)

(fn `UserConstructionScript`)